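; Player hero Blueprint with world-axis movement, mouse-cursor aiming, and punch or gun attacks chosen by HasGun.
; Tick calls EquipGun once when HasGun is true, spawning Gun_bp and attaching it to the mesh's GunSocket.
; Left click moves a spawned MousePointBP marker to the cursor hit, yaws the mesh toward it and fires, or punches when unarmed.
; Movement rotates the mesh unless IsShooting, which movement input clears after a delay.
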(event EventBeginPlay
  (bind _returnvalue (Game|SpawnActorfromClass "/Game/UI/MousePointBP.MousePointBP_C" (Math|Conversions|ToTransform(Vector) (Transformation|GetActorLocation)) "Undefined" 0 0))
  (Variables|Default|SetMouseClickPoint _returnvalue)
  (Variables|/Script/Engine.PlayerController|SetbShowMouseCursor (Game|GetPlayerController 0) true))

(event Collision|EventActorBeginOverlap
  (params (OtherActor :type Actor%20Object%20Reference)))

(event EventTick
  (params (DeltaSeconds :type Float%20%28single-precision%29))
  (if (Variables|Default|GetHasGun)
    (Utilities|FlowControl|DoOnce false
      (:Completed
        (CallFunction|EquipGun)))))

(event Input|ActionEvents|InputActionLeftMouseClicked
  (params (Key :type Key%20Structure :default "AnyKey"))
  (bind _returnvalue (Transformation|GetActorLocation))
  (bind _mouseclickpoint (Variables|Default|GetMouseClickPoint))
  (bind _hasgun (Variables|Default|GetHasGun))
  (bind _arrow (Variables|/Game/UI/MousePointBP.MousePointBP_C|GetArrow _mouseclickpoint))
  (bind _returnvalue_2 (Transformation|GetWorldLocation _arrow))
  (bind _returnvalue_3 (- _returnvalue_2 _returnvalue))
  (bind (_x _y) (Math|Vector|BreakVector _returnvalue_3))
  (bind _returnvalue_4 (Math|Vector|MakeVector _x _y 0.0))
  (bind _returnvalue_5 (Math|Conversions|RotationFromXVector _returnvalue_4))
  (bind (_roll _pitch _yaw) (Math|Rotator|BreakRotator _returnvalue_5))
  (:Pressed
    (if _hasgun
      (Transformation|SetActorLocation (Variables|Default|GetMouseClickPoint) (.Location (Collision|BreakHitResult (.HitResult (Game|Player|GetHitResultUnderCursorbyChannel (Game|GetPlayerController 0) "TraceTypeQuery1" true)))) false false)
      (Transformation|SetWorldRotation (Variables|Character|GetMesh) (Math|Rotator|MakeRotator _roll _pitch (- _yaw 9e+01)) false false)
      (Default|Fire (Variables|Default|GetGun))
      (Variables|Default|SetisShooting true)
      (else
        (Variables|Default|SetisPunching true))))
  (:Released
    (if (not _hasgun)
      (Variables|Default|SetisPunching false))))

(event Input|AxisEvents|InputAxisMoveForward
  (params (AxisValue :type Float%20%28single-precision%29))
  (if (!= AxisValue 0.0)
    (Pawn|Input|AddMovementInput "10.000000, 0, 0" AxisValue false)
    (if (Variables|Default|GetisShooting)
      (Utilities|FlowControl|DoOnce false :!label _label
        (:Completed
          (Utilities|FlowControl|Delay 2.0)
          (Variables|Default|SetisShooting false)
          (goto _label Reset)))
      (else
        (Transformation|SetWorldRotation (Variables|Character|GetMesh) (Math|Rotator|MakeRotator (.Roll (Math|Rotator|BreakRotator (Math|Conversions|RotationFromXVector (Math|Vector|MakeVector AxisValue (stale Input|AxisEvents|InputAxisMoveRight AxisValue) 0.0)))) (.Pitch (Math|Rotator|BreakRotator (Math|Conversions|RotationFromXVector (Math|Vector|MakeVector AxisValue (stale Input|AxisEvents|InputAxisMoveRight AxisValue) 0.0)))) (- (.Yaw (Math|Rotator|BreakRotator (Math|Conversions|RotationFromXVector (Math|Vector|MakeVector AxisValue (stale Input|AxisEvents|InputAxisMoveRight AxisValue) 0.0)))) 9e+01)) false false)))))

(event Input|AxisEvents|InputAxisMoveRight
  (params (AxisValue :type Float%20%28single-precision%29))
  (if (!= AxisValue 0.0)
    (Pawn|Input|AddMovementInput "0,10.000000, 0" AxisValue false)
    (if (Variables|Default|GetisShooting)
      (Utilities|FlowControl|DoOnce false :!label _label
        (:Completed
          (Utilities|FlowControl|Delay 2.0)
          (Variables|Default|SetisShooting false)
          (goto _label Reset)))
      (else
        (Transformation|SetWorldRotation (Variables|Character|GetMesh) (Math|Rotator|MakeRotator (.Roll (Math|Rotator|BreakRotator (Math|Conversions|RotationFromXVector (Math|Vector|MakeVector (stale Input|AxisEvents|InputAxisMoveForward AxisValue) AxisValue 0.0)))) (.Pitch (Math|Rotator|BreakRotator (Math|Conversions|RotationFromXVector (Math|Vector|MakeVector (stale Input|AxisEvents|InputAxisMoveForward AxisValue) AxisValue 0.0)))) (- (.Yaw (Math|Rotator|BreakRotator (Math|Conversions|RotationFromXVector (Math|Vector|MakeVector (stale Input|AxisEvents|InputAxisMoveForward AxisValue) AxisValue 0.0)))) 9e+01)) false false)))))

(fn ConstructionScript)

(fn EquipGun
  (bind _returnvalue (Game|SpawnActorfromClass "/Game/StarterContent/FPWeapon/Mesh/gun_bp.gun_bp_C" (Transformation|GetWorldTransform (Variables|Default|GetGunPosition)) "Undefined" 0 0))
  (bind _output_get (Variables|Default|SetGun _returnvalue))
  (Transformation|AttachComponentToComponent _output_get (Variables|Character|GetMesh) "GunSocket" "SnapToTarget" "SnapToTarget" "KeepWorld" true))